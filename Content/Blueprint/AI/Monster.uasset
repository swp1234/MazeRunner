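; Monster AI character that tracks whether it senses the player and switches between walk and sprint speeds.
; AI Perception updates store or clear SeenPlayer and the IsPlayerInSight flag, without checking that the sensed actor is the player.
; BeginSprint and EndSprint set the movement speed and sprint flag.
; SensePlayer is empty; its older three-direction box-trace sight check is left disconnected and never runs.
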(event `self.ReceiveBeginPlay`
  (set `CharacterMovementComponent.MaxWalkSpeed` (`self.WalkSpeed`) (`self.CharacterMovement`)))

(event `self.ReceiveTick`
  (params (DeltaSeconds :type "Float (single-precision)")))

(event `self.AIPerception.OnTargetPerceptionUpdated`
  (params (Actor :type "Actor Object Reference") (Stimulus :type "AIStimulus Structure"))
  (if Stimulus_bSuccessfullySensed
    (set `self.SeenPlayer` Actor)
    (set `self.IsPlayerInSight` true)
    (else
      (set `self.SeenPlayer` null)
      (set `self.IsPlayerInSight` false))))

(fn `BeginSprint`
  (set `CharacterMovementComponent.MaxWalkSpeed` (`self.SprintSpeed`) (`self.CharacterMovement`))
  (set `self.isSprint` true))

(fn `EndSprint`
  (set `CharacterMovementComponent.MaxWalkSpeed` (`self.WalkSpeed`) (`self.CharacterMovement`))
  (set `self.isSprint` false))

(fn `SensePlayer`
  (returns (IsSeen :type Boolean) (SeenActor :type "Actor Object Reference"))
  (locals (TraceDistance :type "Float (double-precision)" :default 2000.0)))

(fn `UserConstructionScript`)