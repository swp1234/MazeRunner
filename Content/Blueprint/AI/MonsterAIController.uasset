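; AI controller for the Monster pawn that runs its patrol behavior tree and tracks the player it sees.
; BeginPlay copies the monster's patrol points, seeds the blackboard with its wait duration and starts AI_Patrol.
; Every Tick sets TargetPawn to the seen player, or clears it when none is in sight.
; Helper functions return the current patrol location and pick the next index at random, possibly repeating the same point.
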(event `self.ReceiveBeginPlay`
  (bind _asmonster (cast `/Game/Blueprint/AI/Monster` (`self.K2_GetPawn`)))
  (set `self.PatrolPoints` (`/Game/Blueprint/AI/Monster.PatrolPoints` _asmonster))
  (`self.UseBlackboard` "/Game/Blueprint/AI/AIBlackBoard_Monster.AIBlackBoard_Monster")
  (`BlackboardComponent.SetValueAsFloat` (`AIBlueprintHelperLibrary.GetBlackboard` null) "PatrolWaitDuration" (`/Game/Blueprint/AI/Monster.PatrolWaitLocation` _asmonster))
  (`self.RunBehaviorTree` "/Game/Blueprint/AI/AI_Patrol.AI_Patrol"))

(event `self.ReceiveTick`
  (params (DeltaSeconds :type "Float (single-precision)"))
  (bind _returnvalue (`AIBlueprintHelperLibrary.GetBlackboard` null))
  (bind _asmonster (cast `/Game/Blueprint/AI/Monster` (`self.K2_GetPawn`)))
  (if (`/Game/Blueprint/AI/Monster.IsPlayerInSight` _asmonster)
    (`BlackboardComponent.SetValueAsObject` _returnvalue "TargetPawn" (`/Game/Blueprint/AI/Monster.SeenPlayer` _asmonster))
    (else
      (`BlackboardComponent.SetValueAsObject` _returnvalue "TargetPawn" null))))

(fn `GetPatrolLocation`
  (returns (Output :type "Vector Structure"))
  (return (`self.K2_GetActorLocation` (`|GetArrayItem` (`self.PatrolPoints`) (`self.PatrolIndex`)))))

(fn `SetNextPatrolIndex`
  (set `self.PatrolIndex` (mod (+ (`self.PatrolIndex`) (`KismetMathLibrary.RandomIntegerInRange` 0 1000)) (`KismetArrayLibrary.Array_Length` (`self.PatrolPoints`)))))

(fn `UserConstructionScript`)