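; Monster is a character Blueprint with an AI Perception component and functions for switching between walking and sprinting.
; Both perception update events feed one debug print of the Actor name from the target-perception event.
; BeginSprint and EndSprint set the movement component's max walk speed and a sprint flag, but nothing in this file calls them.
; BeginPlay, Tick, overlap and the construction script are empty.
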(event `self.AIPerception.OnTargetPerceptionUpdated`
  (params (Actor :type "Actor Object Reference") (Stimulus :type "AIStimulus Structure"))
  (`KismetSystemLibrary.PrintString` (`KismetSystemLibrary.GetDisplayName` Actor) :!label _label))

(event `self.AIPerception.OnPerceptionUpdated`
  (params (UpdatedActors :type "Array of Actor Object Reference (by ref)"))
  (goto _label))

(fn `BeginSprint`
  (set `CharacterMovementComponent.MaxWalkSpeed` (`self.SprintSpeed`) (`self.CharacterMovement`))
  (set `self.isSrpint` true))

(fn `EndSprint`
  (set `CharacterMovementComponent.MaxWalkSpeed` (`self.WalkSpeed`) (`self.CharacterMovement`))
  (set `self.isSrpint` false))

(fn `UserConstructionScript`)