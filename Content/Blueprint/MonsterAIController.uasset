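; AI controller for the Monster pawn that drives patrolling between the monster's assigned patrol points.
; On BeginPlay it copies those points, writes the monster's patrol wait value to the blackboard and runs the AI_Patrol behavior tree.
; Helpers return the current point's location and advance the index by a random wrapped offset.
; A GoToPatrol event, not called here, moves there and reschedules itself by timer on success.
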(event `self.ReceiveBeginPlay`
  (bind _asmonster (cast `/Game/Blueprint/Monster` (`self.K2_GetPawn`)))
  (set `self.PatrolPoints` (`/Game/Blueprint/Monster.PatrolPoints` _asmonster))
  (`self.UseBlackboard` "/Game/Blueprint/AIBlackBoard_Monster.AIBlackBoard_Monster")
  (`BlackboardComponent.SetValueAsFloat` (`AIBlueprintHelperLibrary.GetBlackboard` null) "PatrolWaitDuration" (`/Game/Blueprint/Monster.PatrolWaitLocation` _asmonster))
  (`self.RunBehaviorTree` "/Game/Blueprint/AI_Patrol.AI_Patrol"))

(event `GoToPatrol`
  (`|AIMoveTo` (`self.K2_GetPawn`) (`self.GetPatrolLocation`) null
    (:`OnSuccess`
      (`self.SetNextPatrolIndex`)
      (`KismetSystemLibrary.K2_SetTimer` null "GoTOPatrol" 1.0))))

(fn `GetPatrolLocation`
  (returns (Output :type "Vector Structure"))
  (return (`self.K2_GetActorLocation` (`|GetArrayItem` (`self.PatrolPoints`) (`self.PatrolIndex`)))))

(fn `SetNextPatrolIndex`
  (bind _returnvalue (`KismetArrayLibrary.Array_Length` (`self.PatrolPoints`)))
  (set `self.PatrolIndex` (mod (+ (`self.PatrolIndex`) (mod (`KismetMathLibrary.RandomIntegerInRange` 0 1000) _returnvalue)) _returnvalue)))

(fn `UserConstructionScript`)